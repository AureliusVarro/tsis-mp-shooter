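; Player inventory component that stores items in one array sized for general, armor and weapon slots.
; PrepareInventory resizes the array and reloads each item from the Items_CSV data table by Id, keeping its quantity.
; OnDeath clears general slots beyond the safe ones, leaving equipment slots untouched.
; Toggle, UI refresh and return-to-base are empty stubs, with older window and rarity-based clearing logic left disconnected.
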(event `self.ToggleInventory`)

(event `self.PrepareInventory`
  (`KismetSystemLibrary.PrintString` "Prep")
  (`KismetArrayLibrary.Array_Resize` (`self.Inventory`) (+ (`self.NumberOfSlots`) (`self.NumberOfArmorSlots`) (`self.NumberOfWeaponSlots`)))
  (for (_array_element _array_index) (`self.Inventory`)
    (bind _returnvalue (`|GetDataTableRow` "/Game/Blueprints/InventorySystem/Data/Items_CSV.Items_CSV" (`.Id_40_E63BDD824733BFD9273D7E989C004799` (break `/Game/Blueprints/InventorySystem/ItemStructure` (break `/Game/Blueprints/InventorySystem/SlotStructure` _array_element))))
      (:`then`
        (`KismetArrayLibrary.Array_Set` (`self.Inventory`) _array_index (make `/Game/Blueprints/InventorySystem/SlotStructure` _returnvalue (`.Quantity_5_727E51AB42326A91E8DF2EA0AA012A25` (break `/Game/Blueprints/InventorySystem/SlotStructure` _array_element))))))))

(event `self.RefreshInventoryUI`)

(fn `onDeath`
  (for _index (range (`self.NumberOfSafeSlots`) (`self.NumberOfSlots`))
    (`KismetArrayLibrary.Array_Set` (`self.Inventory`) _index)))

(fn `onReturnToBase`)