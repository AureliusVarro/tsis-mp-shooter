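; Base inventory component that holds items as an array of quantity-based slots, with empty ToggleInventory and RefreshInventoryUI stubs.
; On BeginPlay it resizes the array to the slot count and fills each slot's item data from the Items_CSV table by Id.
; Adding tops up a partial stack or claims a free slot, recursing on overflow past max stack size.
; It also removes quantities, checks item totals by Id and swaps slots between inventories.
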(event `self.ReceiveBeginPlay`
  (`self.PrepareInventory`))

(fn `AddToInventory`
  (params (ContentToAdd :type "/Game/Blueprints/InventorySystem/SlotStructure Structure"))
  (`KismetSystemLibrary.PrintString` (`KismetStringLibrary.Concat_StrStr` "Trying To Place : " (`KismetStringLibrary.Conv_IntToString` ContentToAdd_Quantity_5_727E51AB42326A91E8DF2EA0AA012A25) " of " (`KismetTextLibrary.Conv_TextToString` (`.Name_2_78B74AAB4A8E1D0D7A6C42AEAEB23F0E` (break `/Game/Blueprints/InventorySystem/ItemStructure` (break `/Game/Blueprints/InventorySystem/SlotStructure` ContentToAdd))))) true true (struct :`G` 0.66 :`B` 1.0 :`A` 1.0) 5.0)
  (if (`.IsStackable_5_719AB5884E6FB41E34FA3999193C4F2D` (break `/Game/Blueprints/InventorySystem/ItemStructure` (break `/Game/Blueprints/InventorySystem/SlotStructure` ContentToAdd)))
    (bind _stackindex (`self.HasPartialStack` (`local.ContentToAdd`))
      (:`True`
        (`self.AddToStack` (`local.ContentToAdd`) _stackindex)
        (return))
      (:`False`
        _)))
  (`self.CreateStack` (`local.ContentToAdd`))
  (return))

(fn `AddToStack`
  (params (SlotStructure :type "/Game/Blueprints/InventorySystem/SlotStructure Structure") (SlotIndex :type Integer))
  (locals (CurrentStackQuantity :type Integer))
  (bind (_itemstructure _quantity) (break `/Game/Blueprints/InventorySystem/SlotStructure` SlotStructure))
  (bind (_slotstructure_itemstructure _slotstructure_quantity) (break `/Game/Blueprints/InventorySystem/SlotStructure` (`local.SlotStructure`)))
  (bind _itemstructure_2 (break `/Game/Blueprints/InventorySystem/SlotStructure` (`local.SlotStructure`)))
  (bind _output (`|GetArrayItem` (`self.Inventory`) SlotIndex))
  (bind (_id _name _thumbnail _description _isstackable _maxstacksize) (break `/Game/Blueprints/InventorySystem/ItemStructure` _itemstructure_2))
  (`KismetSystemLibrary.PrintString` "Adding To Stack")
  (bind _output_get (set `local.CurrentStackQuantity` (`.Quantity_5_727E51AB42326A91E8DF2EA0AA012A25` (break `/Game/Blueprints/InventorySystem/SlotStructure` _output))))
  (bind _returnvalue (+ _output_get _quantity))
  (if (> _returnvalue (`.MaxStackSize_18_FDF18D524BD9D2A8F6F686BB15362EBE` (break `/Game/Blueprints/InventorySystem/ItemStructure` (break `/Game/Blueprints/InventorySystem/SlotStructure` _output))))
    (`KismetArrayLibrary.Array_Set` (`self.Inventory`) (`local.SlotIndex`) (make `/Game/Blueprints/InventorySystem/SlotStructure` _itemstructure_2 _maxstacksize))
    (`self.AddToInventory` (make `/Game/Blueprints/InventorySystem/SlotStructure` _slotstructure_itemstructure (- _slotstructure_quantity (- _maxstacksize (`local.CurrentStackQuantity`)))))
    (return)
    (else
      (`KismetArrayLibrary.Array_Set` (`self.Inventory`) (`local.SlotIndex`) (make `/Game/Blueprints/InventorySystem/SlotStructure` _itemstructure _returnvalue))
      (return))))

(fn `CreateStack`
  (params (ContentToAdd :type "/Game/Blueprints/InventorySystem/SlotStructure Structure"))
  (returns (Success :type Boolean))
  (locals (HasSpace :type Boolean) (`Free Index` :type Integer :default -1))
  (bind (_contenttoadd_itemstructure _contenttoadd_quantity) (break `/Game/Blueprints/InventorySystem/SlotStructure` (`local.ContentToAdd`)))
  (bind _free_index (`local.Free Index`))
  (bind _contenttoadd (`local.ContentToAdd`))
  (bind _free_index_2 (`local.Free Index`))
  (`KismetSystemLibrary.PrintString` (`KismetStringLibrary.Concat_StrStr` "Creating Stack "))
  (for (_array_element _array_index) (`self.Inventory`)
    (if (<= (`.Quantity_5_727E51AB42326A91E8DF2EA0AA012A25` (break `/Game/Blueprints/InventorySystem/SlotStructure` _array_element)) 0)
      (set `local.Free Index` _array_index)
      (set `local.HasSpace` true)
      (break)
      (elif (> _array_index (`self.NumberOfSlots`))
        (break))))
  (if (and (`local.HasSpace`) (>= _free_index_2 0) (< _free_index_2 (`self.NumberOfSlots`)))
    (if (<= (`.Quantity_5_727E51AB42326A91E8DF2EA0AA012A25` (break `/Game/Blueprints/InventorySystem/SlotStructure` _contenttoadd)) (`.MaxStackSize_18_FDF18D524BD9D2A8F6F686BB15362EBE` (break `/Game/Blueprints/InventorySystem/ItemStructure` (break `/Game/Blueprints/InventorySystem/SlotStructure` _contenttoadd))))
      (`KismetArrayLibrary.Array_Set` (`self.Inventory`) _free_index (`local.ContentToAdd`))
      (`KismetSystemLibrary.PrintString` (`KismetStringLibrary.Concat_StrStr` "Added to : " (`KismetStringLibrary.Conv_IntToString` _free_index)))
      (return true)
      (else
        (`KismetArrayLibrary.Array_Set` (`self.Inventory`) (`local.Free Index`) (make `/Game/Blueprints/InventorySystem/SlotStructure` _contenttoadd_itemstructure (`.MaxStackSize_18_FDF18D524BD9D2A8F6F686BB15362EBE` (break `/Game/Blueprints/InventorySystem/ItemStructure` (break `/Game/Blueprints/InventorySystem/SlotStructure` _contenttoadd)))))
        (bind _success (`self.CreateStack` (make `/Game/Blueprints/InventorySystem/SlotStructure` _contenttoadd_itemstructure (- _contenttoadd_quantity (`.MaxStackSize_18_FDF18D524BD9D2A8F6F686BB15362EBE` (break `/Game/Blueprints/InventorySystem/ItemStructure` (break `/Game/Blueprints/InventorySystem/SlotStructure` _contenttoadd)))))))
        (return _success)))
    (else
      (return false))))

(fn `InventoryQuery`
  (params (QueryItemId :type Name) (QueryAmount :type Integer))
  (returns (IsInInventory :type Boolean))
  (locals (RunningTotal :type Integer))
  (for _array_element (`self.Inventory`)
    (if (== (`.Id_40_E63BDD824733BFD9273D7E989C004799` (break `/Game/Blueprints/InventorySystem/ItemStructure` (break `/Game/Blueprints/InventorySystem/SlotStructure` _array_element))) (`local.QueryItemId`))
      (set `local.RunningTotal` (+ (`.Quantity_5_727E51AB42326A91E8DF2EA0AA012A25` (break `/Game/Blueprints/InventorySystem/SlotStructure` _array_element)) (`local.RunningTotal`)))))
  (return (>= (`local.RunningTotal`) (`local.QueryAmount`))))

(fn `PrepareInventory`
  (locals (TempItem :type "/Game/Blueprints/InventorySystem/ItemStructure Structure"))
  (`KismetSystemLibrary.PrintString` "Prep")
  (`KismetArrayLibrary.Array_Resize` (`self.Inventory`) (`self.NumberOfSlots`))
  (for (_array_element _array_index) (`self.Inventory`)
    (bind _output_get (set `local.TempItem` (break `/Game/Blueprints/InventorySystem/SlotStructure` _array_element)))
    (bind _returnvalue (`|GetDataTableRow` "/Game/Blueprints/InventorySystem/Data/Items_CSV.Items_CSV" (break `/Game/Blueprints/InventorySystem/ItemStructure` _output_get))
      (:`then`
        (`KismetArrayLibrary.Array_Set` (`self.Inventory`) _array_index (make `/Game/Blueprints/InventorySystem/SlotStructure` _returnvalue (`.Quantity_5_727E51AB42326A91E8DF2EA0AA012A25` (break `/Game/Blueprints/InventorySystem/SlotStructure` _array_element))))))))

(fn `RefreshInventoryUI`)

(fn `RemoveFromStack`
  (params (Quantity :type Integer) (index :type Integer))
  (bind (_itemstructure _quantity) (break `/Game/Blueprints/InventorySystem/SlotStructure` (`|GetArrayItem` (`self.Inventory`) index)))
  (bind _returnvalue (- _quantity Quantity))
  (if (> _returnvalue 0)
    (`KismetArrayLibrary.Array_Set` (`self.Inventory`) (`local.index`) (make `/Game/Blueprints/InventorySystem/SlotStructure` _itemstructure _returnvalue))
    (else
      (`KismetArrayLibrary.Array_Set` (`self.Inventory`) (`local.index`) (make `/Game/Blueprints/InventorySystem/SlotStructure` (struct :`Name` "NSLOCTEXT(\"[8C7ADA584733AD51434ABABF3DD7130C]\", \"A889138C4594159DE5912CB6B3D17F73\", \"None\")" :`Description` "NSLOCTEXT(\"[8C7ADA584733AD51434ABABF3DD7130C]\", \"C2E76C194CFE527D397877B4A4AC026A\", \"None\")" :`IsStackable` true :`MaxStackSize` 5 :`Rarity` "NewEnumerator0" :`ItemType` "NewEnumerator7"))))))

(fn `SwapItems`
  (params (ThisIndex :type Integer) (FromInventory :type "/Game/Blueprints/InventorySystem/InventoryComponent_Base Object Reference") (FromIndex :type Integer))
  (locals (Temp :type "/Game/Blueprints/InventorySystem/SlotStructure Structure"))
  (bind _inventory (`/Game/Blueprints/InventorySystem/InventoryComponent_Base.Inventory` FromInventory))
  (bind _inventory_2 (`self.Inventory`))
  (set `local.Temp` (`|GetArrayItem` _inventory_2 ThisIndex))
  (`KismetArrayLibrary.Array_Set` _inventory_2 ThisIndex (`|GetArrayItem` _inventory FromIndex))
  (`KismetArrayLibrary.Array_Set` _inventory FromIndex (`local.Temp`)))

(fn `ToggleInventory`)