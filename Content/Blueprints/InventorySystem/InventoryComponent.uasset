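; Child inventory component that prepares the inventory at BeginPlay, handles item additions and refreshes inventory widgets.
; AddToInventory prints a debug string and calls ServerAddToInventory, which runs the parent implementation.
; RefreshInventoryUI calls ServerRefreshUI, which refreshes each valid entry in Widgets.
; ToggleInventory is empty; its old window, input and pause logic remains as unreachable nodes.
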(event `Server AddToInventory`
  (params (`Content to Add` :type "/Game/Blueprints/InventorySystem/SlotStructure Structure"))
  (`parent.AddToInventory` `Content to Add`))

(event `self.ReceiveBeginPlay`
  (`self.PrepareInventory`))

(event `self.ToggleInventory`)

(event `self.RefreshInventoryUI`
  (`self.Server RefreshUI`))

(event `Server RefreshUI`
  (for _array_element (`self.Widgets`)
    (`/Engine/EditorBlueprintResources/StandardMacros.IsValid` (`KismetSystemLibrary.Conv_InterfaceToObject` _array_element)
      (:`Is Valid`
        (`/Game/Blueprints/InventorySystem/IRefreshable.Refresh` _array_element)))))

(fn `AddToInventory`
  (params (ContentToAdd :type "/Game/Blueprints/InventorySystem/SlotStructure Structure"))
  (`KismetSystemLibrary.PrintString` "Inv-child" true true (struct :`R` 1.0 :`G` 0.974541 :`A` 1.0) 5.0)
  (`self.Server AddToInventory` ContentToAdd))